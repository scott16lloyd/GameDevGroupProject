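; Boss character Blueprint for a boss fight, with a melee punch attack, health and an on-screen health bar.
; The Attack event plays a punch montage, gated by an IsAttacking flag until it completes.
; BeginPlay creates the health widget, and Tick refreshes its bar from Health.
; AnyDamage subtracts Health and, at zero or below, disables movement and sets mesh physics simulation off.
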(event EventBeginPlay
  (bind _returnvalue (UserInterface|CreateWidget "/Game/BossFight/WB_BossFightHealth.WB_BossFightHealth_C"))
  (Utilities|FlowControl|Delay 0.0)
  (UserInterface|Viewport|AddtoViewport _returnvalue 100)
  (Variables|Default|SetHealth%20UI _returnvalue))

(event EventTick
  (params (DeltaSeconds :type Float%20%28single-precision%29))
  (Utilities|FlowControl|Delay 0.0)
  (Progress|SetPercent (Variables|/Game/BossFight/WB_BossFightHealth.WB_BossFightHealth_C|GetBossHealthBar (Variables|Default|GetHealth%20UI)) (/ (Variables|Default|Gethealth) 1e+02)))

(event Game|Damage|EventAnyDamage
  (params (Damage :type Float%20%28single-precision%29) (DamageType :type Damage%20Type%20Object%20Reference) (InstigatedBy :type Controller%20Object%20Reference) (DamageCauser :type Actor%20Object%20Reference))
  (Variables|Default|Sethealth (- (Variables|Default|Gethealth) Damage))
  (if (<= (Variables|Default|Gethealth) 0.0)
    (Pawn|Components|CharacterMovement|DisableMovement (Variables|Character|GetCharacterMovement))
    (Physics|SetSimulatePhysics (Variables|Character|GetMesh) false)))

(event EventAttack
  ;[0.15 0.15 0.15 0.5] Attack
  (if (not (Variables|Default|GetisAttacking?))
    (Animation|Montage|PlayMontage (Variables|Character|GetMesh) "/Game/BossFight/Mutant/mutant_punch_Montage.mutant_punch_Montage"
      (:then
        (Variables|Default|SetisAttacking? true))
      (:OnCompleted
        (Variables|Default|SetisAttacking? false)))))

(fn ConstructionScript)